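; VR player pawn with camera-relative movement, 45-degree snap turning, shooting, health and XP leveling.
; Shooting line-traces from the right controller, destroys the hit actor and awards XP into a buffer.
; Tick eases XP toward that buffer and levels up, carrying overflow into a growing threshold until max level.
; At zero health, Tick reveals a plane and reloads the current level after a delay.
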(event EventBeginPlay
  (CallFunction|CalculateXpPercentage))

(event EventTick
  (params (DeltaSeconds :type Float%20%28single-precision%29))
  (if (<= (Variables|Default|GetHealth) 0.0)
    (Development|SetHiddeninGame (Variables|Default|GetPlane) false false)
    (Utilities|FlowControl|Delay 3.0)
    (bind _returnvalue (Game|GetCurrentLevelName true))
    (Game|OpenLevel(byName) (Utilities|String|StringToName _returnvalue))
    (else
      (Variables|Default|SetXp (Math|Conversions|ToFloat(Integer) (Math|Float|Ceil (Math|Interpolation|FInterpTo (Variables|Default|GetXp) (Variables|Default|GetXpBuffer) DeltaSeconds 5.0))))
      (CallFunction|CalculateXpPercentage)
      (if (>= (Variables|Default|GetXp) (Variables|Default|GetXpToLevel))
        (CallFunction|LevelUp)))))

(event Input|ActionEvents|InputActionCameraAngleLeft
  (params (Key :type Key%20Structure :default "None"))
  (:Pressed
    (Transformation|SetActorRotation (Math|Rotator|CombineRotators (Transformation|GetActorRotation self) "0,-45.000000, 0"))))

(event Input|ActionEvents|InputActionShot
  (params (Key :type Key%20Structure :default "None"))
  (bind _rightcontroller (Variables|Default|GetRightController))
  (bind _returnvalue (Transformation|GetWorldLocation _rightcontroller))
  (:Pressed
    (bind _returnvalue_2 (AddComponent|AddAudioComponent false))
    (Audio|Components|Audio|Play _returnvalue_2 0.0)
    (bind _outhit (Collision|LineTraceForObjects _returnvalue (+ _returnvalue (* (Math|Vector|GetForwardVector (Transformation|GetWorldRotation _rightcontroller)) 1.5e+03)) (Variables|Default|GetNewVar_0) false 0 "ForDuration" true "(R=0.745404,G=0.104616,B=0.068478,A=1.000000)" "(R=0.745404,G=0.104616,B=0.068478,A=1.000000)" 1.0))
    (if (Utilities|IsValid (.HitActor (Collision|BreakHitResult _outhit)))
      (Actor|DestroyActor (.HitActor (Collision|BreakHitResult _outhit)))
      (CallFunction|GainXP 3e+02)
      (bind _returnvalue_3 (AddComponent|AddAudioComponent false))
      (Audio|Components|Audio|Play _returnvalue_3 0.0))))

(event Input|ActionEvents|InputActionCameraAngleRight
  (params (Key :type Key%20Structure :default "None"))
  (:Pressed
    (Transformation|SetActorRotation (Math|Rotator|CombineRotators (Transformation|GetActorRotation self) "0,45.000000, 0"))))

(event Input|AxisEvents|InputAxisMoveRight
  (params (AxisValue :type Float%20%28single-precision%29))
  (Transformation|SetActorLocation (Utilities|AddMovement AxisValue (* (Math|Vector|GetRightVector (Variables|Default|GetCamera)) "1.000000,1.000000, 0")) true false))

(event Input|AxisEvents|InputAxisMoveForward
  (params (AxisValue :type Float%20%28single-precision%29))
  (Transformation|SetActorLocation (Utilities|AddMovement AxisValue (* (Math|Vector|GetForwardVector (Variables|Default|GetCamera)) "1.000000,1.000000, 0")) true false))

(fn ConstructionScript
  (Class|PrimitiveComponent|SetUseCCD (Variables|Pawn|GetCapsule) true "None"))

(fn CalculateXpPercentage
  (Variables|Default|SetXpPercentage (/ (Variables|Default|GetXp) (Variables|Default|GetXpToLevel))))

(fn CalculateXpMax
  (Variables|Default|SetXpToLevel (Math|Conversions|ToFloat(Integer) (Math|Float|Ceil (* (Variables|Default|GetXpToLevel) 1.7)))))

(fn GainXP
  (params (Added%20XP :type Float%20%28single-precision%29))
  (Variables|Default|SetXpBuffer (+ Added%20XP (Variables|Default|GetXpBuffer))))

(fn LevelUp
  (if (>= (Variables|Default|GetLevel) (Variables|Default|GetMaxLevel))
    (bind _output_get (Variables|Default|SetXp (Variables|Default|GetXpToLevel)))
    (Variables|Default|SetXpBuffer _output_get)
    (else
      (Math|Integer|IncrementInt (Variables|Default|GetLevel)
        (:%20%20
          (LocalVariables|SetXpRemaining (- (Variables|Default|GetXpBuffer) (Variables|Default|GetXpToLevel)))
          (CallFunction|CalculateXpMax)
          (Variables|Default|SetXp 0.0)
          (Variables|Default|SetXpBuffer 0.0)
          (CallFunction|GainXP (LocalVariables|GetXpRemaining))
          (bind _returnvalue (AddComponent|AddAudioComponent false))
          (Audio|Components|Audio|Play _returnvalue 0.0))))))

(fn LoseHealth
  (Variables|Default|SetHealth (- (Variables|Default|GetHealth) 0.0025)))

(fn Die
  (bind _asplayer_controller (Utilities|Casting|CastToPlayerController (Pawn|GetController)))
  (CameraFades|StartCameraFade :self (Variables|/Script/Engine.PlayerController|GetPlayerCameraManager _asplayer_controller) :ToAlpha 1.0 :Duration 9.0 :bShouldFadeAudio true)
  (bind _returnvalue (Game|GetCurrentLevelName true))
  (Game|OpenLevel(byName) (Utilities|String|StringToName _returnvalue)))