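; Enemy spawner actor that repeatedly spawns BP_Enemy AI at its own location at an accelerating rate.
; A one-shot timer starts on BeginPlay and re-arms itself after each spawn, shortening the interval by a fixed step every time.
; Each spawn also adds a new audio component and plays it.
; The interval has no lower bound.
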(event Custom|SpawnEnemy
  (AI|SpawnAIFromClass "/Game/Enemies/BP_Enemy.BP_Enemy_C" 0 (Transformation|GetActorLocation) "0, 0, 0" false 0)
  (bind _returnvalue (AddComponent|AddAudioComponent false))
  (Audio|Components|Audio|Play _returnvalue 0.0)
  (bind _output_get (Variables|Default|Settime (- (Variables|Default|Gettime) 0.15)))
  (Utilities|Time|SetTimerbyEvent (delegate Custom|SpawnEnemy) _output_get))

(event EventBeginPlay
  (Utilities|Time|SetTimerbyEvent (delegate Custom|SpawnEnemy) (Variables|Default|Gettime)))

(fn ConstructionScript)