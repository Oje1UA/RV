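; Enemy pawn that chases the player and costs them health on reaching them.
; Every tick it looks up a BP_Pawn_VR, falling back to BP_Pawn_W when none exists, and reissues AI MoveTo toward it with stop-on-overlap.
; A successful move calls LoseHealth on that player pawn.
; On Destroyed it calls RemoveTickPrerequisiteActor with no actor specified.
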(event EventDestroyed
  (Class|Actor|RemoveTickPrerequisiteActor))

(event EventTick
  (params (DeltaSeconds :type Float%20%28single-precision%29))
  (bind _self self)
  (bind _returnvalue (Actor|GetActorOfClass "/Game/Player/BP_Pawn_VR.BP_Pawn_VR_C"))
  (if (Utilities|IsValid _returnvalue)
    (AI|AIMoveTo _self "0, 0, 0" _returnvalue 5.0 true
      (:OnSuccess
        (Default|LoseHealth _returnvalue)))
    (else
      (bind _returnvalue_2 (Actor|GetActorOfClass "/Game/Player/BP_Pawn_W.BP_Pawn_W_C"))
      (AI|AIMoveTo _self "0, 0, 0" _returnvalue_2 5.0 true
        (:OnSuccess
          (Default|LoseHealth _returnvalue_2))))))

(fn ConstructionScript)